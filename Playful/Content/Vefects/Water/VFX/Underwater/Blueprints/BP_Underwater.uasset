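; BP_Underwater is a trigger volume that applies an underwater look and sound while the player is inside it.
; Box overlap events for the player pawn switch a post-process component's blend weight fully on or off and fade the underwater audio cue in or out.
; A timeline that would lerp the blend weight exists but is never triggered, so the visual change is instant while the sound fades.
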(event `self.Box.OnComponentBeginOverlap`
  (params (OverlappedComponent :type "PrimitiveComponent Object Reference") (OtherActor :type "Actor Object Reference") (OtherComp :type "PrimitiveComponent Object Reference") (OtherBodyIndex :type Integer) (bFromSweep :type Boolean) (SweepResult :type "HitResult Structure (by ref)"))
  (if (== OtherActor (`GameplayStatics.GetPlayerPawn` 0))
    (`|ExecutionSequence`
      (:`then_0`
        (set `PostProcessComponent.BlendWeight` 1.0 (`self.PostProcess`)))
      (:`then_1`
        (`AudioComponent.FadeIn` (`self.SFX_Vefects_Water_Underwater_General_Cue`) 0.3 1.0 0.0 "Linear")))))

(event `self.Box.OnComponentEndOverlap`
  (params (OverlappedComponent :type "PrimitiveComponent Object Reference") (OtherActor :type "Actor Object Reference") (OtherComp :type "PrimitiveComponent Object Reference") (OtherBodyIndex :type Integer))
  (if (== OtherActor (`GameplayStatics.GetPlayerPawn` 0))
    (`|ExecutionSequence`
      (:`then_0`
        (set `PostProcessComponent.BlendWeight` 0.0 (`self.PostProcess`)))
      (:`then_1`
        (`AudioComponent.FadeOut` (`self.SFX_Vefects_Water_Underwater_General_Cue`) 0.3 0.0 "Linear")))))

(fn `UserConstructionScript`)