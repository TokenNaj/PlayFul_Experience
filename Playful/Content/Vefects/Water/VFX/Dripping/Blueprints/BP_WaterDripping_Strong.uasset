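; Strong water drip effect actor that fits a dripping mesh, splash Niagara effect and puddle decal to the surface below it.
; The construction script traces down from the actor, moves the splashes and decal to the hit, and stretches the mesh height to the drop distance.
; Splash width and spawn rate follow the mesh's X scale and a rate multiplier.
; On a hit, the puddle decal is destroyed when AddPuddle is off.
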(fn `UserConstructionScript`
  (bind (_returnvalue_x _returnvalue_y _returnvalue_z) (`KismetMathLibrary.BreakVector` (`self.K2_GetActorLocation`)))
  (bind _returnvalue (`self.K2_GetActorLocation`))
  (bind _relativescale3d_x (`KismetMathLibrary.BreakVector` (`SceneComponent.RelativeScale3D` (`self.WaterDrippingMesh`))))
  (bind _relativescale3d_x_2 (`KismetMathLibrary.BreakVector` (`SceneComponent.RelativeScale3D` (`self.DefaultSceneRoot`))))
  (bind _returnvalue_2 (* _relativescale3d_x 20.0))
  (bind (_outhit _returnvalue_3) (`KismetSystemLibrary.LineTraceSingle` _returnvalue (- _returnvalue (0.0 0.0 1000.0)) "TraceTypeQuery1" false (`|MakeArray` self :!type "Actor Object Reference")))
  (if _returnvalue_3
    (`SceneComponent.K2_SetWorldLocation` (`self.NS_Splashes`) (+ (`.Location` (`GameplayStatics.BreakHitResult` _outhit)) (0.0 0.0 1.0)) false false)
    (`SceneComponent.K2_SetWorldLocation` (`self.PuddleDecal`) (`.Location` (`GameplayStatics.BreakHitResult` _outhit)) false false)
    (`SceneComponent.SetRelativeScale3D` (`self.WaterDrippingMesh`) (`KismetMathLibrary.MakeVector` _relativescale3d_x_2 1.0 (/ (- _returnvalue_z (.z (`.Location` (`GameplayStatics.BreakHitResult` _outhit)))) 200.0)))
    (`NiagaraComponent.SetVariableFloat` (`self.NS_Splashes`) "Height" 5.0)
    (`NiagaraComponent.SetVariableFloat` (`self.NS_Splashes`) "Width" _returnvalue_2)
    (`NiagaraComponent.SetVariableFloat` (`self.NS_Splashes`) "SpawnRate" (* _returnvalue_2 (`self.Splashes Spawn Rate Multiplier`)))
    (if (not (`self.Add Puddle`))
      (`ActorComponent.K2_DestroyComponent` (`self.PuddleDecal`)))))