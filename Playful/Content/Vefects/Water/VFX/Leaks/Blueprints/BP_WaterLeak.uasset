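; Water leak effect actor that configures its NSWaterLeak particle component entirely in the construction script, with no active event graph logic.
; It passes the drop spawn rate and the turbulence disc toggle to the effect as parameters.
; A downward visibility line trace from the actor finds the surface below and, on a hit, feeds that point to the effect as its ground location.
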(fn `UserConstructionScript`
  (bind _returnvalue (`self.K2_GetActorLocation`))
  (`FXSystemComponent.SetFloatParameter` (`self.NS_WaterLeak`) "SpawnRate" (`self.WaterDropsSpawnRate`))
  (`FXSystemComponent.SetBoolParameter` (`self.NS_WaterLeak`) "Water Turbulent Disc" (`self.AddWaterTurbulenceDisc`))
  (bind (_outhit _returnvalue_2) (`KismetSystemLibrary.LineTraceSingle` _returnvalue (+ _returnvalue (0.0 0.0 -1000.0)) "TraceTypeQuery1"))
  (if _returnvalue_2
    (`FXSystemComponent.SetVectorParameter` (`self.NS_WaterLeak`) "GroundLocation" (`.Location` (`GameplayStatics.BreakHitResult` _outhit)))))