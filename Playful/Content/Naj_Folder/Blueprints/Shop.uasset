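; Shop actor that toggles a shop menu when its Interaction event fires, pausing the game while the menu is open.
; The Shop_Widget is created on demand and kept in ShopMenu for reuse.
; The game's pause state decides open or close, switching viewport display, mouse cursor and input mode together.
; Several unconnected copies of the open and close logic remain in the graph and never run.
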(event `/Game/Naj_Folder/Blueprints/Player_Interface.Interaction`
  (bind _returnvalue (`GameplayStatics.GetPlayerController` 0))
  (bind _shop_menu (`self.Shop Menu`))
  (`/Engine/EditorBlueprintResources/StandardMacros.IsValid` null
    (:`Is Valid`
      _)
    (:`Is Not Valid`
      (bind _returnvalue_2 (`|CreateWidget` "/Game/Naj_Folder/Widget/Shop_Widget.Shop_Widget_C"))
      (set `self.Shop Menu` _returnvalue_2)))
  (if (`GameplayStatics.IsGamePaused`)
    (`Widget.RemoveFromParent` _shop_menu)
    (`GameplayStatics.SetGamePaused` false)
    (set `PlayerController.bShowMouseCursor` false _returnvalue)
    (`WidgetBlueprintLibrary.SetInputMode_GameOnly` _returnvalue)
    (else
      (`UserWidget.AddToViewport` _shop_menu 0)
      (`GameplayStatics.SetGamePaused` true)
      (set `PlayerController.bShowMouseCursor` true _returnvalue)
      (`WidgetBlueprintLibrary.SetInputMode_GameAndUIEx` _returnvalue _shop_menu "LockInFullscreen" false))))

(fn `UserConstructionScript`)